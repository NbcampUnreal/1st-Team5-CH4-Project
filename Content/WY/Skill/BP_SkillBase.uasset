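; Base skill actor that spawns a timed VFX actor, plays a start sound and runs area checks around itself.
; On BeginPlay it sets timers for skill duration and a looping effect interval; the finish event clears timers and destroys the actor.
; DrawShape sphere-overlaps pawns and passes hits to CallOnOverlapEffect, with optional debug drawing.
; A damage helper, not called here, messages enemy combat components, judging enemies by team or instigator.
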(event Custom|OnSkill
  ;[0.15 0.15 0.15 0.5] 스킬 동작
  (bind _returnvalue (Utilities|Time|SetTimerbyEvent (EventDispatchers|CreateEvent :!event Custom|OnSkillFinish) (Variables|ControllValue|GetSkillDuration)))
  (Variables|Timer|SetSkillOnTimer _returnvalue)
  (Utilities|Time|SetTimerbyEvent (EventDispatchers|CreateEvent :!event Custom|DrawShape) (Variables|ControllValue|GetSkillEffectIntaval) true)
  (Variables|Timer|SetDamagedTimer ""))

(event Custom|SpawnFX
  ;[0.15 0.15 0.15 0.5] Fx가져오기
  (CallFunction|OnSkill)
  (bind _returnvalue (CallFunction|SpawnVFX (Variables|Effect|GetVFX) (Variables|Effect|GetVFX%20Type)))
  (Variables|Effect|SetVFX_Actor _returnvalue)
  (CallFunction|StartSoundPlay))

(event Custom|OnSkillFinish
  ;[0.15 0.15 0.15 0.5] 스킬 동작
  (Utilities|Time|ClearandInvalidateTimerbyHandle (Variables|Timer|GetSkillOnTimer))
  (Utilities|Time|ClearandInvalidateTimerbyHandle (Variables|Timer|GetDamagedTimer))
  (Actor|DestroyActor))

(event Custom|DrawShape
  (bind _returnvalue (Transformation|GetActorLocation))
  ;[0.15 0.15 0.15 0.5] OnSkillEvent
  (if (Variables|Default|GetDrawDebug)
    (Rendering|Debug|DrawDebugSphere _returnvalue (Variables|ControllValue|GetSkillCollisionRadius) 12 "(R=0.000000,G=1.000000,B=0.086815,A=1.000000)" 1.0))
  (bind (_outactors _returnvalue_2) (Collision|SphereOverlapActors _returnvalue (Variables|ControllValue|GetSkillCollisionRadius) (Utilities|Array|MakeArray "ObjectTypeQuery3") "/Script/Engine.Pawn" (select (Variables|Default|GetIgnoreInstigator) (Utilities|Array|MakeArray (Game|GetInstigator)) 0)))
  (if _returnvalue_2
    (Default|CallOnOverlapEffect _outactors)))

(event EventBeginPlay
  (CallFunction|SpawnFX))

(fn ConstructionScript)

(fn IAmmoGetType
  (return "NewEnumerator2"))

(fn HaveCombatComponent
  (params (Actor :type Actor%20Object%20Reference))
  (return (Utilities|IsValid (CallFunction|FGetCombatStateComponent Actor))))

(fn IsEnemyActor
  (params (OverlapActor :type Object%20Object%20Reference))
  (bind _ascharacter (Utilities|Casting|CastToCharacter OverlapActor))
  (LocalVariables|SetOverlapCharacter _ascharacter)
  (if (CallFunction|HaveTeamGame)
    (if (!= (CallFunction|FGetActorTeam (Variables|Actor|GetInstigator)) (CallFunction|FGetActorTeam (LocalVariables|GetOverlapCharacter)))
      (return true)
      (else
        (return false)))
    (elif (!= (Variables|Actor|GetInstigator) OverlapActor)
      (return true)
      (else
        (return false)))))

(fn SpawnVFX
  (params (VFX :type Object%20Object%20Reference) (VFX_Type :type E_VFXType%20Enum :default "NewEnumerator0"))
  (bind _returnvalue (Components|GetOwner))
  (Utilities|IsValid _returnvalue
    (:Is%20Valid
      (Variables|Effect|GetVFX_Actor
        (:then)
        (:else
          (bind _returnvalue_2 (Game|SpawnActorfromClass :Class "/Game/WY/Skill/BP_VFX.BP_VFX_C" :CollisionHandlingOverride "Undefined" :TransformScaleMethod "MultiplyWithRoot" :Owner _returnvalue :VFX_Type VFX_Type :VFX VFX :Duration (Variables|ControllValue|GetSkillDuration) :SocketName (Variables|Default|GetSocket%20Name) :Instigator (.AsCBP%20Default (Utilities|Casting|CastToCBP_Default _returnvalue))))
          (return _returnvalue_2))))))

(fn StartSoundPlay
  (Audio|PlaySoundatLocation (Variables|Effect|GetStartSound) (Transformation|GetActorLocation (Game|GetInstigator)) "0, 0, 0" 1.0 1.0 0.0 0 0 0 0))

(fn SandDamage
  (params (OverlapActor :type Actor%20Object%20Reference))
  (if (and (CallFunction|HaveCombatComponent OverlapActor) (CallFunction|IsEnemyActor OverlapActor))
    (Class|BPIComponentsCombat|IDamageReceived(Message) (CallFunction|FGetCombatStateComponent OverlapActor) (Variables|Damage|GetDamageConfig) (Game|GetInstigator) (Variables|Damage|GetReaction))))

(fn RangeCollision)

(fn HaveTeamGame
  (return (!= (CallFunction|FGetActorTeam (Game|GetInstigator)) -1)))