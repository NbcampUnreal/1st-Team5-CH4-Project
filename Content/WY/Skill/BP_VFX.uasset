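; Skill VFX actor that plays a Niagara or Cascade effect for a set duration.
; On BeginPlay it spawns a system asset at its transform, or takes an existing component and attaches at a named socket, then starts a cleanup timer.
; Every tick it moves the effect component to the Instigator's location, preferring Niagara.
; DestroyVFX removes the components and actor, and a helper sets Niagara float scale parameters.
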(event Custom|DestroyVFX
  (Utilities|FlowControl|Sequence
    (:then_0
      (bind _as_niagara_particle_system_component (Variables|Default|GetAs%20Niagara%20Particle%20System%20Component)
        (:then
          (Components|Activation|Deactivate _as_niagara_particle_system_component)
          (Components|DestroyComponent _as_niagara_particle_system_component))
        (:else)))
    (:then_1
      (bind _as_cascade_particle_system_component (Variables|Default|GetAs%20Cascade%20Particle%20System%20Component)
        (:then
          (Components|Activation|Deactivate _as_cascade_particle_system_component)
          (Components|DestroyComponent _as_cascade_particle_system_component))
        (:else)))
    (:then_2
      (Actor|DestroyActor))))

(event Custom|UpdateVFXLocation
  (bind _returnvalue (Game|GetInstigator))
  (bind _returnvalue_2 (Transformation|GetActorLocation _returnvalue))
  (Utilities|IsValid _returnvalue
    (:Is%20Valid
      (bind _as_niagara_particle_system_component (Variables|Default|GetAs%20Niagara%20Particle%20System%20Component)
        (:then
          (Transformation|SetWorldLocation _as_niagara_particle_system_component _returnvalue_2 false false))
        (:else
          (bind _as_cascade_particle_system_component (Variables|Default|GetAs%20Cascade%20Particle%20System%20Component)
            (:then
              (Transformation|SetWorldLocation _as_cascade_particle_system_component _returnvalue_2 false false))
            (:else)))))))

(event EventBeginPlay
  (Variables|Default|GetVFX
    (:then
      ;[0.15 0.15 0.15 0.5] 컴포넌트 가져오기
      (switch Utilities|FlowControl|Switch|SwitchonE_VFXType (Variables|Default|GetVFX_Type)
        (:NewEnumerator0
          (bind _asniagara_system (Utilities|Casting|CastToNiagaraSystem (Variables|Default|GetVFX)))
          (Variables|Default|SetAs%20Niagara%20Particle%20System%20Component (CallFunction|SpawnNiagaraComponent _asniagara_system))
          (CallFunction|DestroyTimer))
        (:NewEnumerator2
          (bind _asparticle_system (Utilities|Casting|CastToParticleSystem (Variables|Default|GetVFX)))
          (Variables|Default|SetAs%20Cascade%20Particle%20System%20Component (CallFunction|SpawnParticleComponent _asparticle_system))
          (CallFunction|DestroyTimer))
        (:NewEnumerator3
          (bind _asniagara_particle_system_component (Utilities|Casting|CastToNiagaraComponent (Variables|Default|GetVFX)))
          (bind _output_get (Variables|Default|SetAs%20Niagara%20Particle%20System%20Component _asniagara_particle_system_component))
          (CallFunction|AttacheBone _output_get)
          (CallFunction|DestroyTimer))
        (:NewEnumerator4
          (bind _ascascade_particle_system_component (Utilities|Casting|CastToParticleSystemComponent (Variables|Default|GetVFX)))
          (bind _output_get_2 (Variables|Default|SetAs%20Cascade%20Particle%20System%20Component _ascascade_particle_system_component))
          (CallFunction|AttacheBone _output_get_2)
          (CallFunction|DestroyTimer))))
    (:else)))

(event EventTick
  (params (DeltaSeconds :type Float%20%28single-precision%29))
  (CallFunction|UpdateVFXLocation))

(fn ConstructionScript)

(fn AttacheBone
  (params (Parent :type Scene%20Component%20Object%20Reference))
  (Transformation|AttachComponentToComponent Parent (Variables|Default|GetSocketName) "KeepRelative" "KeepRelative" "KeepRelative" true))

(fn SpawnParticleComponent
  (params (EmitterTemplate :type Particle%20System%20Object%20Reference))
  (bind _returnvalue (Transformation|GetActorTransform))
  (bind (_location _rotation _scale) (Math|Transform|BreakTransform _returnvalue))
  (bind _returnvalue_2 (Effects|SpawnEmitteratLocation EmitterTemplate _location _rotation _scale))
  (return _returnvalue_2))

(fn SpawnNiagaraComponent
  (params (SystemTemplate :type Niagara%20System%20Object%20Reference))
  (bind _returnvalue (Transformation|GetActorTransform))
  (bind (_location _rotation _scale) (Math|Transform|BreakTransform _returnvalue))
  (bind _returnvalue_2 (Niagara|SpawnSystematLocation SystemTemplate _location _rotation _scale))
  (return _returnvalue_2))

(fn DestroyTimer
  (Utilities|Time|SetTimerbyEvent (EventDispatchers|CreateEvent :!event Custom|DestroyVFX) (Variables|Default|GetDuration)))

(fn SetNiagaraScale
  (params (Scale :type Float%20%28double-precision%29) (ParameterName :type Name))
  (Niagara|SetNiagaraVariable(Float) (Variables|Default|GetAs%20Niagara%20Particle%20System%20Component) ParameterName Scale))