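; BP_ShieldSkill is a shield skill actor that makes its instigating CBP_Default character invincible and keeps a visual effect on it.
; On BeginPlay it enables an invincibility type through the character's CombatStateHandling server update; this file never turns it off.
; Each tick it moves VFXActor to the instigator's location.
; CalculRadiusDistance returns the point at SkillCollisionRadius from the skill toward a given enemy.
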(event Custom|UpdateLocation
  (bind _returnvalue (Game|GetInstigator))
  (bind _vfx_actor (Variables|Default|GetVFX_Actor)
    (:then
      (Utilities|IsValid _returnvalue
        (:Is%20Valid
          (Transformation|SetActorLocation _vfx_actor (Transformation|GetActorLocation _returnvalue) false false))))
    (:else)))

(event EventBeginPlay
  (|CallParentFunction)
  (bind _ascbp_default (Utilities|Casting|CastToCBP_Default (Variables|Default|GetInstigator)))
  (Default|SERVERUpdateInvincibleState (Variables|/Game/BMMCSystem/Blueprints/Character/BP_MainCharacter.BP_MainCharacter_C|GetCombatStateHandling _ascbp_default) true "NewEnumerator1"))

(event EventTick
  (params (DeltaSeconds :type Float%20%28single-precision%29))
  (CallFunction|UpdateLocation))

(fn ConstructionScript
  (|CallParentFunction))

(fn CalculRadiusDistance
  (params (EnemyActor :type Actor%20Object%20Reference))
  (bind _returnvalue (Transformation|GetActorLocation))
  (return (+ (* (Math|Vector|Normalize (- (Transformation|GetActorLocation EnemyActor) _returnvalue)) (Variables|Default|GetSkillCollisionRadius)) _returnvalue)))