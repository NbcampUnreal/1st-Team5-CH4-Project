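; Animation notify that spawns a skill actor, set by SkillClass, when the animation reaches the notify, apparently for ranged skills.
; It casts the mesh's owner to CBP_Default and spawns only where that character has authority.
; The skill spawns at the character's location, without its rotation, with the character as both Owner and Instigator.
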(fn ReceivedNotify
  (params (MeshComp :type Skeletal%20Mesh%20Component%20Object%20Reference) (Animation :type Anim%20Sequence%20Base%20Object%20Reference) (EventReference :type Anim%20Notify%20Event%20Reference%20Structure%20%28by%20ref%29))
  (bind _returnvalue (CallFunction|GetOwnerCharacter MeshComp))
  (if (Ability|HasAuthority _returnvalue)
    (Game|SpawnActorfromClass (Variables|Default|GetSkillClass) (Math|Conversions|ToTransform(Vector) (Transformation|GetActorLocation _returnvalue)) "Undefined" "MultiplyWithRoot" _returnvalue _returnvalue)
    (return false)))

(fn GetOwnerCharacter
  (params (MeshComp :type Actor%20Component%20Object%20Reference))
  (bind _ascbp_default (Utilities|Casting|CastToCBP_Default (Components|GetOwner MeshComp)))
  (return _ascbp_default))