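; Anim notify that spawns a skill actor on every member of the caster's team, for team-wide skills.
; It runs only with authority and reads the owner's team index to pick the Team A or Team B player list from BP_GS_MultiPlayer.
; Each actor spawns at a teammate's location, owned by that teammate with the caster as instigator.
; Without a team (index -1, solo mode), it spawns one actor on the caster.
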(fn ReceivedNotify
  (params (MeshComp :type Skeletal%20Mesh%20Component%20Object%20Reference) (Animation :type Anim%20Sequence%20Base%20Object%20Reference) (EventReference :type Anim%20Notify%20Event%20Reference%20Structure%20%28by%20ref%29))
  (bind _returnvalue (Components|GetOwner MeshComp))
  (bind _ascbp_default (Utilities|Casting|CastToCBP_Default _returnvalue))
  ;[0.15 0.15 0.15 0.5] 팀전분별
  (if (Ability|HasAuthority (Components|GetOwner MeshComp))
    (if (CallFunction|HaveTeam MeshComp)
      ;[0.15 0.15 0.15 0.5] 팀이 있을경우
      (bind _asbp_gs_multi_player (Utilities|Casting|CastToBP_GS_MultiPlayer (Game|GetGameState)))
      (for _array_element (Utilities|Select :Index (CallFunction|GetTeamIndex MeshComp) :Option%200 (Variables|/Game/BMMCSystem/Blueprints/GameModes/Multiplayer/BP_GS_MultiPlayer.BP_GS_MultiPlayer_C|GetTeamAPlayers _asbp_gs_multi_player) :Option%201 (Variables|/Game/BMMCSystem/Blueprints/GameModes/Multiplayer/BP_GS_MultiPlayer.BP_GS_MultiPlayer_C|GetTeamBPlayers _asbp_gs_multi_player))
        (Game|SpawnActorfromClass (Variables|Default|GetSkillClass) (Math|Transform|MakeTransform (Transformation|GetActorLocation _array_element) "0, 0, 0" "1.000000,1.000000,1.000000") "AlwaysSpawn" "MultiplyWithRoot" _array_element (.AsCBP%20Default (Utilities|Casting|CastToCBP_Default (Components|GetOwner MeshComp)))))
      (return false)
      (else
        ;[0.15 0.15 0.15 0.5] 개인전
        (Game|SpawnActorfromClass (Variables|Default|GetSkillClass) (Math|Transform|MakeTransform (Transformation|GetActorLocation _ascbp_default) "0, 0, 0" "1.000000,1.000000,1.000000") "Undefined" "MultiplyWithRoot" _ascbp_default _ascbp_default)
        (return false)))))

(fn GetTeamIndex
  (params (MeshComp :type Actor%20Component%20Object%20Reference))
  (return (CallFunction|FGetActorTeam (CallFunction|GetOwnerCharacter MeshComp))))

(fn HaveTeam
  (params (MeshComp :type Actor%20Component%20Object%20Reference))
  (return (!= (CallFunction|GetTeamIndex MeshComp) -1)))