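; Fire arrow projectile Blueprint, a child that specializes inherited projectile behavior.
; On BeginPlay it loads its setup through SetProjectileInfo using the FireArrow name.
; Its AttachToHitActor override always passes false for AttachOnHit to the parent, so attachment is switched off, then deactivates the Niagara arrow trail.
; A delayed downward velocity change is left unconnected and never runs.
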(event Custom|DeactivateTrail
  (Components|Activation|Deactivate (Variables|Default|GetNS_ArrowTrail)))

(event EventBeginPlay
  (CallFunction|SetProjectileInfo "FireArrow"))

(event Collision|EventActorBeginOverlap
  (params (OtherActor :type Actor%20Object%20Reference)))

(event EventTick
  (params (DeltaSeconds :type Float%20%28single-precision%29)))

(fn ConstructionScript
  (|CallParentFunction))

(fn AttachtoHitActor
  (params (HitComp :type Scene%20Component%20Object%20Reference) (Hit :type Hit%20Result%20Structure%20%28by%20ref%29) (AttachOnHit :type Boolean))
  (|CallParentFunction HitComp Hit false)
  (CallFunction|DeactivateTrail)
  (return))