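; Base arrow-style projectile Blueprint that loads its config from DT_Projectiles and launches with a velocity passed through an interface.
; On its first sphere hit it sends damage through combat component interfaces, after excluding the weapon's owner and checking the hit is allowed.
; It can then stick to the struck bone with movement and collision disabled, and starts its lifespan.
; Hits on WorldStatic or Destructible set a RepNotify flag that spawns impact VFX.
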(event OnComponentHit(Sphere)
  (params (HitComponent :type Primitive%20Component%20Object%20Reference) (OtherActor :type Actor%20Object%20Reference) (OtherComp :type Primitive%20Component%20Object%20Reference) (NormalImpulse :type Vector :default "0, 0, 0") (Hit :type Hit%20Result%20Structure%20%28by%20ref%29))
  (if (not (Variables|Default|GetHit))
    (Utilities|IsValid OtherActor
      (:Is%20Valid
        (Variables|Default|SetHit true)
        (CallFunction|SendDamage OtherActor Hit)
        (CallFunction|AttachtoHitActor OtherComp Hit (Variables|Default|GetbAttachOnHit))
        (Actor|SetLifeSpan (Variables|Default|GetIn%20Lifespan%20On%20Hit))
        (if (CallFunction|IsWall OtherComp)
          (Variables|Default|SetHitWall true))))))

(event EventIProjectilesConstruct
  (params (Name :type Name :default "None") (Velocity :type Vector :default "0, 0, 0"))
  (bind _projectilemovement (Variables|Default|GetProjectileMovement))
  (Components|Activation|Activate _projectilemovement false)
  (Variables|/Script/Engine.MovementComponent|SetVelocity _projectilemovement Velocity))

(event EventBeginPlay
  (CallFunction|SetProjectileInfo "BaseArrow"))

(fn ConstructionScript)

(fn SendDamage
  (params (Actor :type Actor%20Object%20Reference) (HitResult :type Hit%20Result%20Structure))
  (bind _actor (CallFunction|GetWeaponOnwer))
  (bind _component (CallFunction|FGetCombatStateComponent Actor))
  (Utilities|IsValid Actor
    (:Is%20Valid
      (Utilities|IsValid _component
        (:Is%20Valid
          (if (!= Actor _actor)
            (bind _component_2 (Class|BPICharacters|GetCombatComp(Message) _actor))
            (bind _return (Class|BPIComponentsCombat|ICanHitShooting(Message) _component_2 _actor Actor))
            (if _return
              (Class|BPIComponentsCombat|IDamageReceived(Message) _component (Utilities|Struct|BreakS_ProjectilesConstruct (Variables|Default|GetProjectileConfig)) _actor (Utilities|Struct|MakeS_DamageReaction HitResult)))))))))

(fn AttachtoHitActor
  (params (HitComp :type Scene%20Component%20Object%20Reference) (Hit :type Hit%20Result%20Structure%20%28by%20ref%29) (AttachOnHit :type Boolean))
  (bind _projectilemovement (Variables|Default|GetProjectileMovement))
  (if AttachOnHit
    (Utilities|IsValid HitComp
      (:Is%20Valid
        (Transformation|AttachComponentToComponent HitComp (.HitBoneName (Collision|BreakHitResult Hit)) "KeepWorld" "KeepWorld" "KeepWorld" true)
        (Variables|/Script/Engine.MovementComponent|SetVelocity _projectilemovement "0, 0, 0")
        (Components|Activation|Deactivate _projectilemovement)
        (Collision|SetCollisionEnabled (Variables|Default|GetSphere) "NoCollision")))))

(fn SpawnWallVFX
  (params (SystemTemplate :type Niagara%20System%20Object%20Reference))
  (Niagara|SpawnSystematLocation SystemTemplate (Transformation|GetWorldLocation (Variables|Default|GetSphere)) (Math|Conversions|RotationFromXVector (* (Transformation|GetActorForwardVector) -1.0)))
  (return))

(fn IsWall
  (params (Actor :type Primitive%20Component%20Object%20Reference))
  (bind _returnvalue (Collision|GetCollisionObjectType Actor))
  (return (or (Utilities|Enum|Equal(Enum) _returnvalue "ECC_WorldStatic") (Utilities|Enum|Equal(Enum) _returnvalue "ECC_Destructible"))))

(fn OnRepHitWall
  (CallFunction|SpawnWallVFX (Variables|Default|GetHitVFX)))

(fn SetProjectileInfo
  (params (Name :type Name))
  (bind _returnvalue (Utilities|GetDataTableRow "/Game/BMMCSystem/Blueprints/DataTables/Additional/DT_Projectiles.DT_Projectiles" Name)
    (:then
      (Variables|Default|SetProjectileConfig _returnvalue))))

(fn GetWeaponOnwer
  (bind _returnvalue (Components|GetOwner))
  (bind (_component _found) (CallFunction|FGetWeaponComponent _returnvalue))
  (if _found
    (bind _actor (Class|BPIComponentsWeapons|IGetWeaponOwner(Message) _component)))
  (return _actor))

(fn IAmmoGetType
  (return "NewEnumerator0"))