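; Tornado skill actor that spawns a particle effect and plays a sound at its instigator, then destroys itself when the skill duration ends.
; A looping timer damages overlapping Characters that have a combat state component, skipping same-team targets, or only the instigator when it has no team.
; SkillMove events shift the actor by local X/Y offsets and print its location.
; It also reports an ammo type through an interface function.
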(event Custom|OnTonado
  (bind _returnvalue (Utilities|Time|SetTimerbyEvent (delegate Custom|OnDamage) (Variables|Default|GetDamageInterval) true))
  (Variables|Default|SetDamagedTimer _returnvalue)
  (bind _returnvalue_2 (Utilities|Time|SetTimerbyEvent (delegate Custom|OnSkillEnd) (Variables|Default|GetSkillDuration)))
  (Variables|Default|SetSkillOnTimer _returnvalue_2)
  (Rendering|SetVisibility (Variables|Default|GetCastCade) true false))

(event Custom|OnSkillEnd
  (Utilities|Time|ClearandInvalidateTimerbyHandle (Variables|Default|GetDamagedTimer))
  (Utilities|Time|ClearandInvalidateTimerbyHandle (Variables|Default|GetSkillOnTimer))
  (Components|DestroyComponent (Variables|Default|GetCastCade))
  (Actor|DestroyActor))

(event Custom|OnDamage
  (for _array_element (Collision|GetOverlappingActors (Variables|Default|GetCollision) "/Script/Engine.Character" :!class /Script/Engine.PrimitiveComponent)
    (if (and (CallFunction|HaveCombatComponent _array_element) (CallFunction|IsTargetActor _array_element))
      (Class|BPIComponentsCombat|IDamageReceived(Message) (CallFunction|FGetCombatStateComponent _array_element) (Variables|Default|GetDamageConfig) (Game|GetInstigator) (Variables|Default|GetReaction)))))

(event Custom|SkillMove
  (params (Value :type Vector%202D%20Structure))
  (bind (_x _y) (Math|Vector2D|BreakVector2D Value))
  (CallFunction|SkillMoveX _x)
  (CallFunction|SkillMoveY _y))

(event Custom|SkillMoveX
  (params (X :type Float%20%28double-precision%29))
  (Transformation|AddActorLocalOffset (Math|Vector|MakeVector X 0.0 0.0) false false)
  (Development|PrintString (Utilities|String|Append "ActorLocation : " (Utilities|String|ToString(Vector) (Transformation|GetActorLocation)))))

(event Custom|SkillMoveY
  (params (Y :type Float%20%28double-precision%29))
  (Transformation|AddActorLocalOffset (Math|Vector|MakeVector 0.0 Y 0.0) false false)
  (Development|PrintString (Utilities|String|Append "ActorLocation : " (Utilities|String|ToString(Vector) (Transformation|GetActorLocation)))))

(event EventBeginPlay
  (bind _returnvalue (AddComponent|AddParticleSystemComponent false))
  (bind _output_get (Variables|Default|SetCastCade _returnvalue))
  (Rendering|SetVisibility _output_get true false)
  (CallFunction|OnTonado)
  (Audio|PlaySoundatLocation (Variables|Default|GetSound) (Transformation|GetActorLocation (Game|GetInstigator)) "0, 0, 0" 1.0 1.0 0.0 0 0 0 0))

(fn ConstructionScript)

(fn IAmmoGetType
  (return "NewEnumerator2"))

(fn HaveCombatComponent
  (params (Actor :type Actor%20Object%20Reference))
  (return (Utilities|IsValid (CallFunction|FGetCombatStateComponent Actor))))

(fn IsTargetActor
  (params (OverlapActor :type Object%20Object%20Reference))
  (bind _ascharacter (Utilities|Casting|CastToCharacter OverlapActor))
  (if (== (CallFunction|FGetActorTeam (Game|GetInstigator)) -1)
    (if (== (Game|GetInstigator) _ascharacter)
      (return false)
      (else
        (return true)))
    (elif (== (CallFunction|FGetActorTeam _ascharacter) (CallFunction|FGetActorTeam (Game|GetInstigator)))
      (return false)
      (else
        (return true)))))